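; BP_Door is an interactable door that swings open away from the player, whichever side they approach from, and closes on the next interaction.
; The Interaction event toggles the closed state and plays or reverses a timeline that lerps the door mesh's relative yaw.
; On opening, a dot product of the door's right vector and the player-to-door direction is stored to choose the swing sign, so closing retraces the same arc.
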(event Custom|OpenCloseDoor
  ;[1 0 1] Opens and closes door using a timeline. It will open the door away from player regardless on which side the player opens the door.
  (if (Variables|Default|GetIsDoorClosed?)
    (Variables|Default|SetIsDoorClosed? false)
    (Variables|Default|SetDotProduct_REF (Math|Vector|DotProduct (Transformation|GetActorRightVector) (Math|Vector|Normalize (- (Transformation|GetActorLocation) (Transformation|GetActorLocation (Variables|Default|GetFPSPlayer_REF))))))
    (bind _alpha (Timeline|OpenCloseDoor_TL Play)
      (:Update
        (Transformation|SetRelativeRotation (Variables|Default|GetSM_Door) (Math|Rotator|MakeRotator 0.0 0.0 (Math|Float|Lerp 0.0 (Math|Float|SelectFloat 85.0 -85.0 (>= (Variables|Default|GetDotProduct_REF) 0.0)) _alpha)) false false)))
    (else
      (Variables|Default|SetIsDoorClosed? true)
      (Timeline|OpenCloseDoor_TL Reverse))))

(event EventBeginPlay
  ;[0 0 1] BeginPlay
  (bind _asbp_first_person_character (Utilities|Casting|CastToBP_FirstPersonCharacter (Game|GetPlayerCharacter 0)))
  (Variables|Default|SetFPSPlayer_REF _asbp_first_person_character))

(event EventInteraction
  ;[1 0 1] When player interacts with object, call event.
  (CallFunction|OpenCloseDoor))

(fn ConstructionScript)