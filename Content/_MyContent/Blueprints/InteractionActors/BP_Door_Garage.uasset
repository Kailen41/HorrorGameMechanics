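; Lockable garage door actor that swings away from the player and auto-closes once they move beyond a set distance.
; Interaction toggles an unlocked door; a locked one compares the last element of the player's Keys to DoorKeyID, then animates key and unlock or shakes.
; Timelines drive door, handle and key motion with sounds.
; A dot product picks swing direction, and a looping timer checks distance.
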(event Custom|OpenCloseDoor
  ;[1 0 1] Opens and closes door using a timeline. It will open the door away from player regardless on which side the player opens the door.
  (CallFunction|FSounds)
  (if (Variables|Door|GetIsDoorClosed?)
    (Variables|Door|SetIsDoorClosed? false)
    (CallFunction|RotateDoorHandle)
    (Variables|Door|SetDotProduct_REF (Math|Vector|DotProduct (Transformation|GetActorRightVector) (Math|Vector|Normalize (- (Transformation|GetActorLocation) (Transformation|GetActorLocation (Variables|Default|GetFPSPlayer_REF))))))
    (bind _alpha (Timeline|OpenCloseDoor_TL Play)
      (:Update
        (Transformation|SetRelativeRotation (Variables|Default|GetSM_Door) (Math|Rotator|MakeRotator 0.0 0.0 (Math|Float|Lerp 0.0 (Math|Float|SelectFloat 85.0 -85.0 (>= (Variables|Door|GetDotProduct_REF) 0.0)) _alpha)) false false)))
    (else
      (Variables|Door|SetIsDoorClosed? true)
      (Timeline|OpenCloseDoor_TL Reverse))))

(event Custom|AutoCloseDoor
  ;[1 0 1] Auto close door by distance of the player.
  (Utilities|Time|SetTimerbyEvent (delegate Custom|DoorAutoClose) 1.0 true))

(event Custom|DoorAutoClose
  ;[1 0 1] Auto close door by distance of the player.
  (if (not (Variables|Door|GetIsDoorClosed?))
    (if (> (Math|Vector|Distance(Vector) (Transformation|GetActorLocation (Variables|Default|GetFPSPlayer_REF)) (Transformation|GetActorLocation)) (Variables|Door|GetCloseDistance))
      (CallFunction|OpenCloseDoor))))

(event Custom|CheckForKey
  ;[1 0 1] Checks to see if the player has a key.
  (for _array_element (Variables|/Game/_MyContent/Blueprints/Characters/BP_FirstPersonCharacter.BP_FirstPersonCharacter_C|GetKeys (Variables|Default|GetFPSPlayer_REF))
    _)
  (if (Utilities|Enum|Equal(Enum) _array_element (Variables|Door|GetDoorKeyID))
    (CallFunction|KeyAnimation)
    (Utilities|FlowControl|Delay 1.0)
    (CallFunction|UnlockDoor)
    (Variables|/Game/_MyContent/Blueprints/Characters/BP_FirstPersonCharacter.BP_FirstPersonCharacter_C|SetHasKey? (Variables|Default|GetFPSPlayer_REF) false)
    (else
      (CallFunction|ShakeDoor))))

(event Custom|RotateDoorHandle
  ;[1 0 1] Rotates the door handle when interacted with the door.
  (bind _alpha (Timeline|DoorHandle_TL PlayFromStart)
    (:Update
      (Transformation|SetRelativeRotation (Variables|Default|GetSM_DoorHandle) (Math|Rotator|MakeRotator 0.0 _alpha 0.0) false false))))

(event Custom|UnlockDoor
  (bind _unlocksound (Variables|Sounds|GetUnlockSound))
  ;[1 0 1] Unlock door with sound
  (Variables|Door|SetIsLocked? false)
  (Audio|PlaySoundatLocation _unlocksound (Transformation|GetWorldLocation (Variables|Default|GetSM_Door)) "0, 0, 0" 1.0 1.0 0.0 0 0 0 0)
  (Utilities|FlowControl|Delay (Variables|/Script/Engine.SoundBase|GetDuration _unlocksound))
  (CallFunction|OpenCloseDoor))

(event Custom|ShakeDoor
  ;[1 0 1] Does a shake door animation with sound and rotates handle
  (CallFunction|RotateDoorHandle)
  (bind _alpha (Timeline|ShakeDoor_TL PlayFromStart)
    (:Update
      (Transformation|SetRelativeRotation (Variables|Default|GetSM_Door) (Math|Rotator|MakeRotator 0.0 0.0 _alpha) false false))
    (:Finished
      (Audio|PlaySoundatLocation (Variables|Sounds|GetLockedSound) (Transformation|GetWorldLocation (Variables|Default|GetSM_Door)) "0, 0, 0" 1.0 1.0 0.0 0 0 0 0))))

(event Custom|KeyAnimation
  (bind _keystartinglocation (Variables|Default|GetKeyStartingLocation))
  ;[1 0 1] Controls key animations. Key turns visable and moves on the Y location and then rotates on the Y. Key's visibility turns off.
  (Rendering|SetVisibility (Variables|Default|GetKey) true false)
  (bind _alpha (Timeline|KeyAnimation01_TL Play)
    (:Update
      (Transformation|SetRelativeLocation (Variables|Default|GetKey) (Math|Vector|MakeVector (.x _keystartinglocation) (Math|Float|Lerp (.y _keystartinglocation) (- (.y _keystartinglocation) 4.0) _alpha) (.z _keystartinglocation)) false false))
    (:Finished
      (bind _alpha_2 (Timeline|KeyAnimation02_TL PlayFromStart)
        (:Update
          (Transformation|SetRelativeRotation (Variables|Default|GetKey) (Math|Rotator|MakeRotator 0.0 _alpha_2 0.0) false false))
        (:Finished
          (Rendering|SetVisibility (Variables|Default|GetKey) false false))))))

(event EventBeginPlay
  ;[0 0 1] BeginPlay
  (bind _asbp_first_person_character (Utilities|Casting|CastToBP_FirstPersonCharacter (Game|GetPlayerCharacter 0)))
  (Variables|Default|SetFPSPlayer_REF _asbp_first_person_character)
  (Variables|Default|SetKeyStartingLocation (Variables|/Script/Engine.SceneComponent|GetRelativeLocation (Variables|Default|GetKey)))
  (CallFunction|AutoCloseDoor))

(event EventInteraction
  ;[1 0 1] When player interacts with object, call event.
  (if (Variables|Door|GetIsLocked?)
    (CallFunction|CheckforKey)
    (else
      (CallFunction|OpenCloseDoor))))

(fn ConstructionScript)

(fn FSounds
  (bind _sm_door (Variables|Default|GetSM_Door))
  (bind _returnvalue (Transformation|GetWorldLocation _sm_door))
  (if (Variables|Door|GetIsLocked?)
    (Audio|PlaySoundatLocation (Variables|Sounds|GetLockedSound) _returnvalue "0, 0, 0" 1.0 1.0 0.0 0 0 0 0)
    (elif (Variables|Door|GetIsDoorClosed?)
      (Audio|PlaySoundatLocation (Variables|Sounds|GetOpenSound) _returnvalue "0, 0, 0" 1.0 1.0 0.0 0 0 0 0)
      (else
        (Audio|PlaySoundatLocation (Variables|Sounds|GetClosedSound) _returnvalue "0, 0, 0" 1.0 1.0 0.0 0 0 0 0)))))