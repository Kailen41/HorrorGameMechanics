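; BP_Key is a key pickup actor that the player collects by interacting with it.
; On BeginPlay it casts player character 0 to BP_FirstPersonCharacter and caches the reference.
; Its Interaction event passes KeyID to that character's AddKeys, then destroys the actor.
; The construction script applies the KeyMesh variable to the static mesh component, so the key's appearance is set through that variable.
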(event EventBeginPlay
  (bind _asbp_first_person_character (Utilities|Casting|CastToBP_FirstPersonCharacter (Game|GetPlayerCharacter 0)))
  (Variables|Default|SetPlayer_REF _asbp_first_person_character))

(event EventInteraction
  (Default|AddKeys (Variables|Default|GetPlayer_REF) (Variables|Default|GetKeyID))
  (Actor|DestroyActor))

(fn ConstructionScript
  (Components|StaticMesh|SetStaticMesh (Variables|Default|GetStaticMesh) (Variables|Default|GetKeyMesh)))